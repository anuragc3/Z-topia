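; BP_Guide is the base-level guide actor that shows progress-dependent dialogue when the player interacts with it.
; BeginPlay moves the player to a fixed spot if the base level was already started, then picks a dialogue array from GI_ztopia's latest completed level.
; Interact opens WP_GuideUI with that text, pauses, and flags the level as started.
; CloseWidget unpauses, but its widget removal relies on WidgetRef, which Interact sets to None.
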(event Custom|Close%20Widget
  (bind _widgetref (Variables|Default|GetWidgetRef))
  ;[1 1 1] Exit/Close Widget
  (Input|SetInputModeGameOnly (Game|GetPlayerController 0) false)
  (Game|SetGamePaused false)
  (Utilities|IsValid _widgetref
    (:Is%20Valid
      (Widget|RemovefromParent _widgetref))))

(event EventBeginPlay
  ;[1 1 1] Set Dialogue based on Level // from Enum
  (Utilities|FlowControl|Sequence
    (:then_0
      ;;[1 1 1] Move Player Location on game start
      (bind _asgi_ztopia (Utilities|Casting|CastToGI_ztopia (Game|GetGameInstance)))
      (if (Variables|/Game/Game/GI_ztopia.GI_ztopia_C|GetBaseLevelStarted _asgi_ztopia)
        (bind _returnvalue (Actor|GetActorOfClass "/Game/Blueprints/Character/BP_Player.BP_Player_C"))
        (Transformation|SetActorLocationAndRotation _returnvalue "900.000000,3400.000000,1752.000000" "0.000000,270.000000,0.000000")))
    (:then_1
      ;;[1 1 1] Get Latest Completed Level from Level Instance
      (bind _asgi_ztopia_2 (Utilities|Casting|CastToGI_ztopia (Game|GetGameInstance)))
      (bind _output_get (Variables|Default|SetDialogueEnum (Variables|/Game/Game/GI_ztopia.GI_ztopia_C|GetLatest_Level_Completed _asgi_ztopia_2)))
      ;;[1 1 1] Set Dialogue based on Level
      (switch Utilities|FlowControl|Switch|SwitchonE_baseDialogues _output_get
        (:NewEnumerator0
          (Variables|Default|SetDialoguesCurrent (Variables|Default|GetDialogueArrayBase)))
        (:NewEnumerator1
          (Variables|Default|SetDialoguesCurrent (Variables|Default|GetDialogueArrayAfterLevel1)))
        (:NewEnumerator2
          (Variables|Default|SetDialoguesCurrent (Variables|Default|GetDialogueArrayAfterLevel2)))
        (:NewEnumerator3
          (Variables|Default|SetDialoguesCurrent (Variables|Default|GetDialogueArrayAfterLevel3)))
        (:NewEnumerator4
          (Variables|Default|SetDialoguesCurrent (Variables|Default|GetDialogueArrayAfterLevel4)))
        (:NewEnumerator5
          (Variables|Default|SetDialoguesCurrent (Variables|Default|GetDialogueArrayAfterLevelFinal)))))))

(event Collision|EventActorBeginOverlap
  (params (OtherActor :type Actor%20Object%20Reference)))

(event EventInteract
  (params (CharacterPickingUp :type BP%20Player%20Object%20Reference))
  ;[1 1 1] Interact // Call Widget with current level's text
  (bind _returnvalue (UserInterface|CreateWidget "/Game/Blueprints/UI/BaseLevel/WP_GuideUI.WP_GuideUI_C" 0 (Variables|Default|GetDialoguesCurrent)))
  (Variables|Default|SetWidgetRef 0)
  (UserInterface|Viewport|AddtoViewport _returnvalue 1)
  (Input|SetInputModeUIOnly (Game|GetPlayerController 0) 0 "DoNotLock" false)
  (Game|SetGamePaused true)
  (bind _asgi_ztopia (Utilities|Casting|CastToGI_ztopia (Game|GetGameInstance)))
  (Variables|/Game/Game/GI_ztopia.GI_ztopia_C|SetBaseLevelStarted _asgi_ztopia true))

(fn ConstructionScript)