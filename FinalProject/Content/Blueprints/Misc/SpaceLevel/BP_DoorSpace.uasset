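; BP_DoorSpace is an interactable space-level door that can be locked.
; BeginPlay caches the door mesh's relative transform, and Interact toggles the door by destroying the mesh component to open it and re-creating it at that transform to close it.
; When locked, the key check is hardcoded false, so Interact always shows a temporary WP_InfoPopUp locked message instead of toggling.
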(event EventInteract
  (params (CharacterPickingUp :type BP%20Player%20Object%20Reference))
  (if (Variables|Default|GetLocked?)
    ;[1 1 1] Does user have key
    (if false
      ;[1 1 1] Door Open Close Logic
      (if (Variables|Default|GetOpen?) :!label _label
        (bind _returnvalue (AddComponent|AddStaticMeshComponent false (Variables|Default|GetDoor%20Position)))
        (bind _output_get (Variables|Default|SetDoor _returnvalue))
        (Components|StaticMesh|SetStaticMesh _output_get "/Game/Assets/Synty/PolygonSciFiSpace/Meshes/Buildings/SM_Bld_Wall_Doorframe_Door_02.SM_Bld_Wall_Doorframe_Door_02")
        (else
          (Components|DestroyComponent (Variables|Default|GetDoor))))
      (Variables|Default|SetOpen? (not (Variables|Default|GetOpen?)))
      (else
        ;[1 1 1] Locked Message
        (bind _returnvalue_2 (UserInterface|CreateWidget "/Game/Blueprints/UI/BaseLevel/WP_InfoPopUp.WP_InfoPopUp_C" 0 (Variables|Default|GetDoorLockedMessage)))
        (UserInterface|Viewport|AddtoViewport _returnvalue_2 0)
        (Utilities|FlowControl|Delay 2.0)
        (Widget|RemovefromParent _returnvalue_2)))
    (else
      (goto _label))))

(event EventBeginPlay
  (Variables|Default|SetDoor%20Position (Transformation|GetRelativeTransform (Variables|Default|GetDoor))))

(fn ConstructionScript)