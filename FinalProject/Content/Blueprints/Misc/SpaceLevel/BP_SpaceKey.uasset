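; BP_SpaceKey is a key pickup actor that, when interacted with, adds its Key value to the interacting character's KeyRing and destroys itself.
; When BP_Player enters the RangeOfPickup component, a WP_InfoPopUp widget shows text built from the key's room, message and value.
; The popup is removed after a short delay or when the player leaves the range.
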(event OnComponentBeginOverlap(rangeOfPickup)
  (params (OverlappedComponent :type Primitive%20Component%20Object%20Reference) (OtherActor :type Actor%20Object%20Reference) (OtherComp :type Primitive%20Component%20Object%20Reference) (OtherBodyIndex :type Integer) (bFromSweep :type Boolean) (SweepResult :type Hit%20Result%20Structure%20%28by%20ref%29))
  (Utilities|Casting|CastToBP_Player OtherActor)
  (bind _returnvalue (UserInterface|CreateWidget "/Game/Blueprints/UI/BaseLevel/WP_InfoPopUp.WP_InfoPopUp_C" 0 (Utilities|Text|ToText(String) (Utilities|String|Append (Utilities|String|Append (Variables|Default|GetKeyRoom) "'s key, ") (Utilities|String|Append (Variables|Default|GetKeyMessage) (Utilities|String|ToString(Integer) (Variables|Default|GetKey)))))))
  (UserInterface|Viewport|AddtoViewport _returnvalue 0)
  (Utilities|FlowControl|Delay 2.0)
  (Widget|RemovefromParent _returnvalue))

(event OnComponentEndOverlap(rangeOfPickup)
  (params (OverlappedComponent :type Primitive%20Component%20Object%20Reference) (OtherActor :type Actor%20Object%20Reference) (OtherComp :type Primitive%20Component%20Object%20Reference) (OtherBodyIndex :type Integer))
  (Utilities|Casting|CastToBP_Player OtherActor)
  (Widget|RemovefromParent (stale OnComponentBeginOverlap(rangeOfPickup) _returnvalue)))

(event EventBeginPlay)

(event Collision|EventActorBeginOverlap
  (params (OtherActor :type Actor%20Object%20Reference)))

(event EventTick
  (params (DeltaSeconds :type Float%20%28single-precision%29)))

(event EventInteract
  (params (CharacterPickingUp :type BP%20Player%20Object%20Reference))
  (Utilities|Array|Add (Variables|/Game/Blueprints/Character/BP_Player.BP_Player_C|GetKeyRing CharacterPickingUp) (Variables|Default|GetKey))
  (Actor|DestroyActor self))

(fn ConstructionScript)