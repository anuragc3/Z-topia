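; BP_GateFake is a fake level gate that teleports the player to a set location and rotation on trigger overlap.
; It spawns a dead zombuter and a "Loading Bay" key, then runs pause, teleport, reverse fade and unpause from one Sequence.
; The Delays have nothing after them, so unpausing and fade-widget removal happen immediately.
; SetGameInstanceData only casts the game instance; its level-progression switch is unconnected.
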(event OnComponentBeginOverlap(LevelTrigger)
  (params (OverlappedComponent :type Primitive%20Component%20Object%20Reference) (OtherActor :type Actor%20Object%20Reference) (OtherComp :type Primitive%20Component%20Object%20Reference) (OtherBodyIndex :type Integer) (bFromSweep :type Boolean) (SweepResult :type Hit%20Result%20Structure%20%28by%20ref%29))
  ;[1 1 1] Enter Level Level
  (Utilities|Casting|CastToBP_Player OtherActor)
  (if true
    (Utilities|FlowControl|Sequence
      (:then_0
        ;;[1 1 1] Spawn dead zombuter and key
        (Game|SpawnActorfromClass "/Game/Blueprints/Misc/SpaceLevel/BP_ZombuterDead.BP_ZombuterDead_C" (Math|Transform|MakeTransform (Variables|Default|GetSpawn%20Transform%20Location) "0, 0, 0" "1.000000,1.000000,1.000000") "Undefined" "MultiplyWithRoot" 0 0)
        (bind _returnvalue (Game|SpawnActorfromClass "/Game/Blueprints/Misc/SpaceLevel/BP_SpaceKey.BP_SpaceKey_C" (Math|Transform|MakeTransform (Variables|Default|GetKeyLocation) "0, 0, 0" "1.000000,1.000000,1.000000") "Undefined" "MultiplyWithRoot" 0 0))
        (Variables|/Game/Blueprints/Misc/SpaceLevel/BP_SpaceKey.BP_SpaceKey_C|SetKey _returnvalue 6666)
        (Variables|/Game/Blueprints/Misc/SpaceLevel/BP_SpaceKey.BP_SpaceKey_C|SetKeyRoom _returnvalue "Loading Bay")
        (Input|SetInputModeUIOnly (Game|GetPlayerController 0) 0 "DoNotLock" false)
        (Game|SetGamePaused true))
      (:then_1
        ;;[1 1 1] Animation
        (bind _returnvalue_2 (Actor|GetActorOfClass "/Game/Blueprints/Character/BP_Player.BP_Player_C"))
        (Transformation|SetActorLocationAndRotation _returnvalue_2 (Variables|Default|GetNew%20Location) "0.000000,180.000000,0.000000")
        (Utilities|FlowControl|Delay 0.5))
      (:then_2
        ;;[1 1 1] Player transport + unfade
        (bind _returnvalue_3 (UserInterface|CreateWidget "/Game/Blueprints/UI/WP_LevelFadeReverse.WP_LevelFadeReverse_C"))
        (UserInterface|Viewport|AddtoViewport _returnvalue_3 0)
        (Default|FadeAnimation _returnvalue_3)
        (Utilities|FlowControl|Delay 0.5))
      (:then_3
        ;;[1 1 1] Unpause Player
        (Input|SetInputModeGameOnly (Game|GetPlayerController 0) false)
        (Game|SetGamePaused false)
        (Widget|RemovefromParent _returnvalue_3)))))

(event Collision|EventActorBeginOverlap
  (params (OtherActor :type Actor%20Object%20Reference)))

(fn ConstructionScript)

(fn SetGameInstanceData
  ;[1 1 1] Set Game Instance values at teleport // Technically only need one portal
  (Utilities|Casting|CastToGI_ztopia (Game|GetGameInstance)))