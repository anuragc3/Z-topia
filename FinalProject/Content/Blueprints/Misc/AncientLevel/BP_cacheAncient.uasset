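; Interactable cache for the Ancient level that the player activates once to count toward their cache total.
; The first interaction increments the interacting character's AncientLevelCache, marks the cache as used and toggles its Beacon's visibility.
; BeginPlay also toggles the Beacon, so activation reverses that initial state.
; Later interactions show a temporary pop-up widget telling the player to find the next cache.
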(event EventBeginPlay
  (Rendering|ToggleVisibility (Variables|Default|Getbeacon) true))

(event Collision|EventActorBeginOverlap
  (params (OtherActor :type Actor%20Object%20Reference)))

(event EventTick
  (params (DeltaSeconds :type Float%20%28single-precision%29)))

(event EventInteract
  (params (CharacterPickingUp :type BP%20Player%20Object%20Reference))
  (if (not (Variables|Default|Getcached))
    (Variables|/Game/Blueprints/Character/BP_Player.BP_Player_C|SetAncientLevelCache CharacterPickingUp (+ (Variables|/Game/Blueprints/Character/BP_Player.BP_Player_C|GetAncientLevelCache CharacterPickingUp) 1))
    (Variables|Default|Setcached true)
    (Rendering|ToggleVisibility (Variables|Default|Getbeacon) true)
    (else
      (bind _returnvalue (UserInterface|CreateWidget "/Game/Blueprints/UI/BaseLevel/WP_InfoPopUp.WP_InfoPopUp_C" 0 "Cache already activated!. Find the next one. Quick bozo!"))
      (UserInterface|Viewport|AddtoViewport _returnvalue 0)
      (Utilities|FlowControl|Delay 3.0)
      (Widget|RemovefromParent _returnvalue))))

(fn ConstructionScript)