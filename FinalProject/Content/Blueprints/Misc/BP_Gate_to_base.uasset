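; BP_Gate_to_base is a gate that sends the player back to the base level.
; When BP_Player overlaps LevelTrigger, it plays a music cue, shows the WP_LevelFade fade widget, then opens BaseLevel after a short delay.
; A separate SetGameInstanceData function, not called within this Blueprint, advances LatestLevelCompleted in GI_ztopia and, except on the last step, sets the base portal's next level name.
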(event OnComponentBeginOverlap(LevelTrigger)
  (params (OverlappedComponent :type Primitive%20Component%20Object%20Reference) (OtherActor :type Actor%20Object%20Reference) (OtherComp :type Primitive%20Component%20Object%20Reference) (OtherBodyIndex :type Integer) (bFromSweep :type Boolean) (SweepResult :type Hit%20Result%20Structure%20%28by%20ref%29))
  ;[1 1 1] Enter Level Level
  (Utilities|Casting|CastToBP_Player OtherActor)
  ;;[1 1 1] Animation
  (Audio|PlaySound2D "/Game/StarterContent/Audio/Starter_Music01.Starter_Music01" 1.0 1.0 0.0 0 0)
  (bind _returnvalue (UserInterface|CreateWidget "/Game/Blueprints/UI/WP_LevelFade.WP_LevelFade_C"))
  (UserInterface|Viewport|AddtoViewport _returnvalue 0)
  (Default|FadeAnimation _returnvalue)
  (Utilities|FlowControl|Delay 0.5)
  ;;[1 1 1] Open Level
  (Game|OpenLevel(byName) (Variables|Default|GetBaseLevel)))

(event Collision|EventActorBeginOverlap
  (params (OtherActor :type Actor%20Object%20Reference)))

(fn ConstructionScript)

(fn SetGameInstanceData
  ;[1 1 1] Set Game Instance values at teleport // Technically only need one portal
  (bind _asgi_ztopia (Utilities|Casting|CastToGI_ztopia (Game|GetGameInstance)))
  (bind _output_get (Variables|Default|SetAs%20GI%20Ztopia _asgi_ztopia))
  (switch Utilities|FlowControl|Switch|SwitchonE_baseDialogues (Variables|/Game/Game/GI_ztopia.GI_ztopia_C|GetLatest_Level_Completed _output_get)
    (:NewEnumerator0
      ;;[1 1 1] Set Level Value in Dialogues ENUM
      (Variables|/Game/Game/GI_ztopia.GI_ztopia_C|SetLatest_Level_Completed (Variables|Default|GetAs%20GI%20Ztopia) "NewEnumerator1")
      ;;[1 1 1] Set Next level of portal
      (Variables|/Game/Game/GI_ztopia.GI_ztopia_C|SetBaseLevel_to_NextLevelValue (Variables|Default|GetAs%20GI%20Ztopia) "Level2"))
    (:NewEnumerator1
      (Variables|/Game/Game/GI_ztopia.GI_ztopia_C|SetLatest_Level_Completed (Variables|Default|GetAs%20GI%20Ztopia) "NewEnumerator2")
      (Variables|/Game/Game/GI_ztopia.GI_ztopia_C|SetBaseLevel_to_NextLevelValue (Variables|Default|GetAs%20GI%20Ztopia) "Level3"))
    (:NewEnumerator2
      (Variables|/Game/Game/GI_ztopia.GI_ztopia_C|SetLatest_Level_Completed (Variables|Default|GetAs%20GI%20Ztopia) "NewEnumerator3")
      (Variables|/Game/Game/GI_ztopia.GI_ztopia_C|SetBaseLevel_to_NextLevelValue (Variables|Default|GetAs%20GI%20Ztopia) "Level4"))
    (:NewEnumerator3
      (Variables|/Game/Game/GI_ztopia.GI_ztopia_C|SetLatest_Level_Completed (Variables|Default|GetAs%20GI%20Ztopia) "NewEnumerator4")
      (Variables|/Game/Game/GI_ztopia.GI_ztopia_C|SetBaseLevel_to_NextLevelValue (Variables|Default|GetAs%20GI%20Ztopia) "Level5"))
    (:NewEnumerator4
      (Variables|/Game/Game/GI_ztopia.GI_ztopia_C|SetLatest_Level_Completed (Variables|Default|GetAs%20GI%20Ztopia) "NewEnumerator5"))))