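; Master weapon Blueprint that provides a hitscan Fire event.
; Fire calls a one-shot animation on WeaponModel, then line traces on the Visibility channel from its location along its right vector, rather than forward.
; The hit actor receives the weapon's Damage through ApplyDamage, with no check on the trace result.
; Persistent debug drawing of the trace is left on, and construction and other events are empty.
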(event EventBeginPlay)

(event Collision|EventActorBeginOverlap
  (params (OtherActor :type Actor%20Object%20Reference)))

(event EventTick
  (params (DeltaSeconds :type Float%20%28single-precision%29)))

(event EventFire
  (bind _weaponmodel (Variables|Default|GetWeaponModel))
  (bind _returnvalue (Transformation|GetWorldLocation _weaponmodel))
  (Components|Animation|PlayAnimation (Variables|Default|GetWeaponModel) 0 false)
  (bind _outhit (Collision|LineTraceByChannel _returnvalue (+ _returnvalue (* (Math|Vector|GetRightVector _weaponmodel) 1e+04)) "TraceTypeQuery1" false 0 "Persistent"))
  (Game|Damage|ApplyDamage (.HitActor (Collision|BreakHitResult _outhit)) (Variables|Default|GetDamage) 0 0 "/Script/Engine.DamageType"))

(fn ConstructionScript)