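; B_PickUpItemParent is the base actor for world items that are picked up into an inventory on overlap.
; When an overlapping actor implements PickUpItemInterface and is not itself a pickup subclass, it receives the item's class, icon, stack size, name, description and usage through PickUpItemMessage.
; The pickup then destroys itself, leaving the receiver to handle the item without any cast to a concrete class.
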(event EventBeginPlay)

(event Collision|EventActorBeginOverlap
  (params (OtherActor :type Actor%20Object%20Reference))
  (if (Utilities|DoesObjectImplementInterface OtherActor "/Game/Blueprints/Inventory/PickUpItemInterface.PickUpItemInterface_C")
    (if (not (Utilities|ClassIsChildOf (Utilities|GetClass OtherActor) "B_PickUpItemParent_C"))
      (Class|PickUpItemInterface|PickUpItem(Message) OtherActor (Variables|Default|GetItemClass) (Variables|Default|GetItemIcon) (Variables|Default|GetStackSize) (Variables|Default|GetItemName) (Variables|Default|GetItemDescription) (Variables|Default|GetUsage))
      (Actor|DestroyActor))))

(fn ConstructionScript)