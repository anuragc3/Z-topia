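; Health pickup actor that heals the player when they walk into its box collision.
; On overlap by BP_Player it calls IncrementHealth, prints the new health and destroys itself.
; IncrementHealth adds a fixed amount clamped to max health.
; At full health it only prints an inventory message, as the AddItemToInventoryMain call is left unconnected, yet the pickup is still destroyed.
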(event OnComponentBeginOverlap(Box)
  (params (OverlappedComponent :type Primitive%20Component%20Object%20Reference) (OtherActor :type Actor%20Object%20Reference) (OtherComp :type Primitive%20Component%20Object%20Reference) (OtherBodyIndex :type Integer) (bFromSweep :type Boolean) (SweepResult :type Hit%20Result%20Structure%20%28by%20ref%29))
  ;[1 1 1] Increment Health
  (bind _asbp_player (Utilities|Casting|CastToBP_Player OtherActor))
  (CallFunction|IncrementHealth _asbp_player)
  (Development|PrintString (Utilities|String|ToString(Float) (Variables|/Game/Blueprints/Character/BP_Player.BP_Player_C|GetPlayerHealth _asbp_player)))
  (Actor|DestroyActor))

(event EventBeginPlay)

(event Collision|EventActorBeginOverlap
  (params (OtherActor :type Actor%20Object%20Reference)))

(event EventTick
  (params (DeltaSeconds :type Float%20%28single-precision%29)))

(fn ConstructionScript)

(fn IncrementHealth
  (params (BP_Player :type BP%20Player%20Object%20Reference))
  (bind _output_get (Variables|Default|SetBP_Player%20Object BP_Player))
  (if (< (Variables|/Game/Blueprints/Character/BP_Player.BP_Player_C|GetPlayerHealth _output_get) (Variables|/Game/Blueprints/Character/BP_Player.BP_Player_C|GetMAX_HEALTH _output_get))
    (Variables|/Game/Blueprints/Character/BP_Player.BP_Player_C|SetPlayerHealth (Variables|Default|GetBP_Player%20Object) (Math|Float|Clamp(Float) (+ (Variables|/Game/Blueprints/Character/BP_Player.BP_Player_C|GetPlayerHealth (Variables|Default|GetBP_Player%20Object)) 15.0) 0.0 (Variables|/Game/Blueprints/Character/BP_Player.BP_Player_C|GetMAX_HEALTH (Variables|Default|GetBP_Player%20Object))))
    (else
      (Development|PrintString "Add To Inventory"))))