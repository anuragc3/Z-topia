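; BP_Zombie is a zombie spawner that starts on BeginPlay and spawns walking or running zombies at its Scene component's transform.
; A random roll picks WalkingZombie half the time; otherwise a second roll spawns RunningZombie or nothing.
; After each spawn, the Spawner event waits a fixed delay and calls itself again.
; The loop stops permanently when the second roll spawns nothing.
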(event Custom|spawner
  (bind _returnvalue (Math|Random|RandomIntegerinRange 0 1))
  (bind _scene (Variables|Default|GetScene))
  (if (== _returnvalue 0)
    (Game|SpawnActorfromClass "/Game/Blueprints/Enemy/MainClasses/WalkingZombie.WalkingZombie_C" (Transformation|GetWorldTransform _scene) "AdjustIfPossibleButDontSpawnIfColliding" "MultiplyWithRoot" 0 0)
    (Utilities|FlowControl|Delay 1e+01)
    (CallFunction|Spawner)
    (elif (== _returnvalue 1)
      (Game|SpawnActorfromClass "/Game/Blueprints/Enemy/MainClasses/RunningZombie.RunningZombie_C" (Transformation|GetWorldTransform _scene) "AdjustIfPossibleButDontSpawnIfColliding" "MultiplyWithRoot" 0 0)
      (Utilities|FlowControl|Delay 1e+01)
      (CallFunction|Spawner))))

(event EventBeginPlay
  (CallFunction|Spawner))

(event Collision|EventActorBeginOverlap
  (params (OtherActor :type Actor%20Object%20Reference)))

(event EventTick
  (params (DeltaSeconds :type Float%20%28single-precision%29)))

(fn ConstructionScript)