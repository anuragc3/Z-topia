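; Password-locked door actor for the dive bar elevator.
; Box overlap by BP_Player enables input on the actor; leaving disables it and removes the password widget.
; E runs a FlipFlop, so only alternate presses show WB_PasswordDiveBarElevator with cursor and UI input, while the door is closed.
; OpenDoor and CloseWidget events restore game-only input; OpenDoor also yaws the door via timeline and sets DoorOpened.
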(event OnComponentBeginOverlap(Box)
  (params (OverlappedComponent :type Primitive%20Component%20Object%20Reference) (OtherActor :type Actor%20Object%20Reference) (OtherComp :type Primitive%20Component%20Object%20Reference) (OtherBodyIndex :type Integer) (bFromSweep :type Boolean) (SweepResult :type Hit%20Result%20Structure%20%28by%20ref%29))
  (Utilities|Casting|CastToBP_Player OtherActor)
  (Input|EnableInput (Game|GetPlayerController 0)))

(event OnComponentEndOverlap(Box)
  (params (OverlappedComponent :type Primitive%20Component%20Object%20Reference) (OtherActor :type Actor%20Object%20Reference) (OtherComp :type Primitive%20Component%20Object%20Reference) (OtherBodyIndex :type Integer))
  (bind _returnvalue (Game|GetPlayerController 0))
  (Utilities|Casting|CastToBP_Player OtherActor)
  (Input|DisableInput (Game|GetPlayerController 0))
  (Widget|RemovefromParent (Variables|Default|GetPassword_Widget))
  (Input|SetInputModeGameOnly _returnvalue false)
  (Variables|/Script/Engine.PlayerController|SetbShowMouseCursor _returnvalue false))

(event Custom|OpenDoor
  (bind _returnvalue (Game|GetPlayerController 0))
  (Input|SetInputModeGameOnly _returnvalue false)
  (Variables|/Script/Engine.PlayerController|SetbShowMouseCursor _returnvalue false)
  (Widget|RemovefromParent (Variables|Default|GetPassword_Widget))
  (bind _door_animation (Timeline|Timeline Play)
    (:Update
      (Transformation|SetRelativeRotation (Variables|Default|GetDoor) (Math|Rotator|MakeRotator 0.0 0.0 _door_animation) false false)
      (Variables|Default|SetdoorOpened true))))

(event Custom|Close%20Widget
  (bind _returnvalue (Game|GetPlayerController 0))
  (Widget|RemovefromParent (Variables|Default|GetPassword_Widget))
  (Input|SetInputModeGameOnly _returnvalue false)
  (Variables|/Script/Engine.PlayerController|SetbShowMouseCursor _returnvalue false))

(event EventBeginPlay)

(event Collision|EventActorBeginOverlap
  (params (OtherActor :type Actor%20Object%20Reference)))

(event EventTick
  (params (DeltaSeconds :type Float%20%28single-precision%29)))

(event Input|KeyboardEvents|E
  (params (Key :type Key%20Structure :default "None"))
  (bind _returnvalue (Game|GetPlayerController 0))
  (:Pressed
    (Utilities|FlowControl|FlipFlop
      (:A
        (if (not (Variables|Default|GetdoorOpened))
          (bind _returnvalue_2 (UserInterface|CreateWidget "/Game/Blueprints/UI/passWordUI/WB_PasswordDiveBarElevator.WB_PasswordDiveBarElevator_C"))
          (bind _output_get (Variables|Default|SetPassword_Widget _returnvalue_2))
          (UserInterface|Viewport|AddtoViewport _output_get 0)
          (Input|SetInputModeGameandUI _returnvalue _output_get "DoNotLock" true false)
          (Variables|/Script/Engine.PlayerController|SetbShowMouseCursor _returnvalue true))))))

(fn ConstructionScript)